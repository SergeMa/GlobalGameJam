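; BP_DamageTaken is a floating text actor in the bot AI folder that, by its name, marks damage taken.
; On BeginPlay it sets DamageText to a random text emoticon or an empty string, with no damage number.
; Each Tick interpolates it toward a point above its current location, so the target moves with it and the text keeps rising.
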(event EventBeginPlay
  (Rendering|Components|TextRender|SetText (Variables|Default|GetDamageText) (.OutItem (Utilities|Array|Random (Utilities|Array|MakeArray (Utilities|Text|ToText(String) ":(") (Utilities|Text|ToText(String) ">:(") (Utilities|Text|ToText(String) ":c") (Utilities|Text|ToText(String) ":|") (Utilities|Text|ToText(String) ">:)") "")))))

(event Collision|EventActorBeginOverlap
  (params (OtherActor :type Actor%20Object%20Reference)))

(event EventTick
  (params (DeltaSeconds :type Float%20%28single-precision%29))
  (bind _returnvalue (Transformation|GetActorLocation))
  (bind (_x _y _z) (Math|Vector|BreakVector _returnvalue))
  (Transformation|SetActorLocation (Math|Interpolation|VInterpTo _returnvalue (Math|Vector|MakeVector _x _y (+ _z 3e+02)) DeltaSeconds 1.0) false false))

(fn ConstructionScript)